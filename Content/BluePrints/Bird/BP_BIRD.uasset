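; BP_BIRD is a bird actor that glides back and forth along the world Y axis.
; Tick accumulates elapsed time into T and subtracts a sine-scaled step from the current location using a swept move.
; The sine acts as a per-frame velocity not scaled by delta time, so travel distance depends on frame rate.
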(event `self.ReceiveTick`
  (params (DeltaSeconds :type "Float (single-precision)"))
  (set `self.t` (+ DeltaSeconds (`self.t`)))
  (`self.K2_SetActorLocation` (- (`self.K2_GetActorLocation`) (`KismetMathLibrary.MakeVector` 0.0 (* (`KismetMathLibrary.Sin` (* (`self.t`) 1.0)) 9.0))) true))

(fn `UserConstructionScript`)