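; BP_Truck is a cargo truck that sways back and forth, then drives away and scores the debris loaded in it.
; Tick moves it along Y in a sine motion for a minute, then steadily toward negative Y, using swept, per-frame steps not scaled by delta time.
; Past a Y threshold, it sets CargoScore once from the count of physics-body BP_Debris actors overlapping CargoOverlapBox, with -1 meaning unscored.
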(event `self.ReceiveBeginPlay`
  (set `self.cargoScore` -1))

(event `self.ReceiveTick`
  (params (DeltaSeconds :type "Float (single-precision)"))
  (bind _output_get (set `self.t` (+ DeltaSeconds (`self.t`))))
  (if (> _output_get 60.0)
    (`self.MoveTruckAway`)
    (if (and (< (.y (`self.K2_GetActorLocation`)) -1200.0) (< (`self.cargoScore`) 0))
      (`self.CalculateCargoScore`))
    (else
      (`self.OscillateTruckPosition`))))

(fn `CalculateCargoScore`
  (bind _cargooverlapbox (`self.CargoOverlapBox`))
  (bind _outactors (`KismetSystemLibrary.ComponentOverlapActors` _cargooverlapbox (`SceneComponent.K2_GetComponentToWorld` _cargooverlapbox) (`|MakeArray` "ObjectTypeQuery4" :!type "EObjectTypeQuery Enum") "/Game/Debris/Blueprints/BP_Debris.BP_Debris_C"))
  (set `self.cargoScore` (* (`KismetArrayLibrary.Array_Length` _outactors) 100)))

(fn `MoveTruckAway`
  (`self.K2_SetActorLocation` (- (`self.K2_GetActorLocation`) (`KismetMathLibrary.MakeVector` 0.0 5.0)) true))

(fn `OscillateTruckPosition`
  (`self.K2_SetActorLocation` (- (`self.K2_GetActorLocation`) (`KismetMathLibrary.MakeVector` 0.0 (* (`KismetMathLibrary.Sin` (* (`self.t`) 1.0)) 5.0))) true))

(fn `UserConstructionScript`)