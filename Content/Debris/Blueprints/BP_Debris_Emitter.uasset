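; BP_Debris_Emitter is an actor that continuously spawns debris boxes at its own location.
; Tick counts down a timer and, when it runs out, calls SpawnDebris and resets the timer to a fixed interval of a few seconds.
; SpawnDebris creates a BP_Debris_Box using the emitter's transform.
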(event `self.ReceiveTick`
  (params (DeltaSeconds :type "Float (single-precision)"))
  (bind _output_get (set `self.timeTillNextEmit` (- (`self.timeTillNextEmit`) DeltaSeconds)))
  (if (< _output_get 0.0)
    (`self.SpawnDebris`)
    (set `self.timeTillNextEmit` 2.5)))

(fn `SpawnDebris`
  (`|SpawnActorFromClass` "/Game/Debris/Blueprints/BP_Debris_Box.BP_Debris_Box_C" (`self.GetTransform`) "Undefined" "MultiplyWithRoot" null null))

(fn `UserConstructionScript`)