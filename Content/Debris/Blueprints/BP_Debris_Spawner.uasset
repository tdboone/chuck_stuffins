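; Debris spawner that keeps its spawn area supplied with random household and street props, such as furniture, appliances and hydrants.
; Tick runs a short repeating countdown that calls SpwnNewDebris.
; That function checks the Box for physics-body BP_Debris actors and, if none overlap, spawns one of eleven subclasses at SpawnPoint.
; Spawning adjusts position if possible and is skipped if still colliding.
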(event `self.ReceiveBeginPlay`
  (bind _output_get (set `self.checkFrequency` 0.75))
  (set `self.checkCounter` _output_get))

(event `self.ReceiveTick`
  (params (DeltaSeconds :type "Float (single-precision)"))
  (bind _output_get (set `self.checkCounter` (- (`self.checkCounter`) DeltaSeconds)))
  (if (< _output_get 0.0)
    (set `self.checkCounter` (`self.checkFrequency`))
    (`self.SpwnNewDebris`)))

(fn `SpwnNewDebris`
  (bind _box (`self.Box`))
  (bind (_outactors _returnvalue) (`KismetSystemLibrary.ComponentOverlapActors` _box (`SceneComponent.K2_GetComponentToWorld` _box) (`|MakeArray` "ObjectTypeQuery4" :!type "EObjectTypeQuery Enum") "/Game/Debris/Blueprints/BP_Debris.BP_Debris_C"))
  (if (not _returnvalue)
    (`|SpawnActorFromClass` (select `int` (`KismetMathLibrary.RandomInteger` 11) :`0` "/Game/Debris/Blueprints/BP_Debris_Box.BP_Debris_Box_C" :`1` "/Game/Debris/Blueprints/BP_Debris_Toilet.BP_Debris_Toilet_C" :`2` "/Game/Debris/Blueprints/BP_Debris_Bookshelf.BP_Debris_Bookshelf_C" :`3` "/Game/Debris/Blueprints/BP_Debris_Casket.BP_Debris_Casket_C" :`4` "/Game/Debris/Blueprints/BP_Debris_TV.BP_Debris_TV_C" :`5` "/Game/Debris/Blueprints/BP_Debris_Hydrant.BP_Debris_Hydrant_C" :`6` "/Game/Debris/Blueprints/BP_Debris_Chair.BP_Debris_Chair_C" :`7` "/Game/Debris/Blueprints/BP_Debris_Pouf.BP_Debris_Pouf_C" :`8` "/Game/Debris/Blueprints/BP_Debris_Cupboard.BP_Debris_Cupboard_C" :`9` "/Game/Debris/Blueprints/BP_Debris_Bath.BP_Debris_Bath_C" :`10` "/Game/Debris/Blueprints/BP_Debris_Oven.BP_Debris_Oven_C" :!type "Actor Class Reference") (`SceneComponent.K2_GetComponentToWorld` (`self.SpawnPoint`)) "AdjustIfPossibleButDontSpawnIfColliding" "MultiplyWithRoot" null null)))

(fn `UserConstructionScript`)